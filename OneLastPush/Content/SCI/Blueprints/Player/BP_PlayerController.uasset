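; Player controller that routes input and UI interface calls to the inventory and interaction systems.
; Hotbar, container, item-move, stack-split and vendor actions forward to InventoryMaster server calls, with inventory, container and vendor screens toggling cursor and pawn input.
; Interact input drives the character's interaction component, supporting instant or timed holds based on the target's trigger time.
; BeginPlay adds the input mapping and retries inventory initialization on a looping timer until it succeeds.
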(event `ResetInteraction (Server)`
  (params (InteractionComponent :type "/Game/SCI/Blueprints/Components/BPC_Interact Object Reference"))
  ;[1 1 1] Interaction
  (`/Game/SCI/Blueprints/Components/BPC_Interact.ResetInteraction` InteractionComponent))

(event `self.ReceiveBeginPlay`
  ;[1 1 1] Setup Inventory Component
  (bind _returnvalue (`KismetSystemLibrary.K2_SetTimerDelegate` (delegate `GetPlayerState`) 0.1 true))
  (set `self.InitTimer` _returnvalue)
  (`self.InitController`))

(event `/Game/SCI/Blueprints/Interfaces/BPI_PlayerController.UpdateInteractUI_BPI`
  (params (Timer :type "Float (double-precision)"))
  ;[1 1 1] Interaction
  (message `/Game/SCI/Blueprints/Interfaces/BPI_HUD.UpdateInteractUI_BPI` (`self.GetHUD`) Timer))

(event `GetPlayerState`
  ;[1 1 1] Setup Inventory Component
  (bind _asbp_player_state (cast `/Game/SCI/Blueprints/Player/BP_PlayerState` (`self.PlayerState`)))
  (bind _success (`/Game/SCI/Blueprints/Components/BPC_InventoryMaster.InitComponent` (`self.InventoryMaster`) _asbp_player_state self (`self.K2_GetPawn`) (`self.GetHUD`)))
  (if _success
    (`KismetSystemLibrary.K2_ClearAndInvalidateTimerHandle` (`self.InitTimer`))))

(event `EnhancedInput|/Game/SCI/Blueprints/Input/Actions/IA_Interact`
  (params (ActionValue :type Boolean) (ElapsedSeconds :type "Float (double-precision)") (TriggeredSeconds :type "Float (double-precision)") (InputAction :type "InputAction Object Reference" :default "/Game/SCI/Blueprints/Input/Actions/IA_Interact.IA_Interact"))
  ;[1 1 1] Interact
  (:`Triggered`
    (bind _returnvalue (== (stale _triggertime) 0.0))
    (if (not _returnvalue)
      (`self.Interact` false ElapsedSeconds :!label _label)))
  (:`Started`
    (bind _triggertime (`self.GetInteractionTime`))
    (if _returnvalue
      (goto _label)))
  (:`Completed`
    (`self.Interact` true)))

(event `EnhancedInput|/Game/SCI/Blueprints/Input/Actions/IA_Hotbar_1`
  (params (ActionValue :type Boolean) (ElapsedSeconds :type "Float (double-precision)") (TriggeredSeconds :type "Float (double-precision)") (InputAction :type "InputAction Object Reference" :default "/Game/SCI/Blueprints/Input/Actions/IA_Hotbar_1.IA_Hotbar_1"))
  ;[1 1 1] Hotbar Inputs
  (:`Started`
    (`/Game/SCI/Blueprints/Components/BPC_InventoryMaster.UseHotbarSlot (Server)` (`self.InventoryMaster`) 0)))

(event `EnhancedInput|/Game/SCI/Blueprints/Input/Actions/IA_Hotbar_5`
  (params (ActionValue :type Boolean) (ElapsedSeconds :type "Float (double-precision)") (TriggeredSeconds :type "Float (double-precision)") (InputAction :type "InputAction Object Reference" :default "/Game/SCI/Blueprints/Input/Actions/IA_Hotbar_5.IA_Hotbar_5"))
  ;[1 1 1] Hotbar Inputs
  (:`Started`
    (`/Game/SCI/Blueprints/Components/BPC_InventoryMaster.UseHotbarSlot (Server)` (`self.InventoryMaster`) 4)))

(event `EnhancedInput|/Game/SCI/Blueprints/Input/Actions/IA_Hotbar_2`
  (params (ActionValue :type Boolean) (ElapsedSeconds :type "Float (double-precision)") (TriggeredSeconds :type "Float (double-precision)") (InputAction :type "InputAction Object Reference" :default "/Game/SCI/Blueprints/Input/Actions/IA_Hotbar_2.IA_Hotbar_2"))
  ;[1 1 1] Hotbar Inputs
  (:`Started`
    (`/Game/SCI/Blueprints/Components/BPC_InventoryMaster.UseHotbarSlot (Server)` (`self.InventoryMaster`) 1)))

(event `EnhancedInput|/Game/SCI/Blueprints/Input/Actions/IA_Hotbar_6`
  (params (ActionValue :type Boolean) (ElapsedSeconds :type "Float (double-precision)") (TriggeredSeconds :type "Float (double-precision)") (InputAction :type "InputAction Object Reference" :default "/Game/SCI/Blueprints/Input/Actions/IA_Hotbar_6.IA_Hotbar_6"))
  ;[1 1 1] Hotbar Inputs
  (:`Started`
    (`/Game/SCI/Blueprints/Components/BPC_InventoryMaster.UseHotbarSlot (Server)` (`self.InventoryMaster`) 5)))

(event `EnhancedInput|/Game/SCI/Blueprints/Input/Actions/IA_Hotbar_3`
  (params (ActionValue :type Boolean) (ElapsedSeconds :type "Float (double-precision)") (TriggeredSeconds :type "Float (double-precision)") (InputAction :type "InputAction Object Reference" :default "/Game/SCI/Blueprints/Input/Actions/IA_Hotbar_3.IA_Hotbar_3"))
  ;[1 1 1] Hotbar Inputs
  (:`Started`
    (`/Game/SCI/Blueprints/Components/BPC_InventoryMaster.UseHotbarSlot (Server)` (`self.InventoryMaster`) 2)))

(event `EnhancedInput|/Game/SCI/Blueprints/Input/Actions/IA_Hotbar_7`
  (params (ActionValue :type Boolean) (ElapsedSeconds :type "Float (double-precision)") (TriggeredSeconds :type "Float (double-precision)") (InputAction :type "InputAction Object Reference" :default "/Game/SCI/Blueprints/Input/Actions/IA_Hotbar_7.IA_Hotbar_7"))
  ;[1 1 1] Hotbar Inputs
  (:`Started`
    (`/Game/SCI/Blueprints/Components/BPC_InventoryMaster.UseHotbarSlot (Server)` (`self.InventoryMaster`) 6)))

(event `EnhancedInput|/Game/SCI/Blueprints/Input/Actions/IA_Hotbar_4`
  (params (ActionValue :type Boolean) (ElapsedSeconds :type "Float (double-precision)") (TriggeredSeconds :type "Float (double-precision)") (InputAction :type "InputAction Object Reference" :default "/Game/SCI/Blueprints/Input/Actions/IA_Hotbar_4.IA_Hotbar_4"))
  ;[1 1 1] Hotbar Inputs
  (:`Started`
    (`/Game/SCI/Blueprints/Components/BPC_InventoryMaster.UseHotbarSlot (Server)` (`self.InventoryMaster`) 3)))

(event `EnhancedInput|/Game/SCI/Blueprints/Input/Actions/IA_Hotbar_8`
  (params (ActionValue :type Boolean) (ElapsedSeconds :type "Float (double-precision)") (TriggeredSeconds :type "Float (double-precision)") (InputAction :type "InputAction Object Reference" :default "/Game/SCI/Blueprints/Input/Actions/IA_Hotbar_8.IA_Hotbar_8"))
  ;[1 1 1] Hotbar Inputs
  (:`Started`
    (`/Game/SCI/Blueprints/Components/BPC_InventoryMaster.UseHotbarSlot (Server)` (`self.InventoryMaster`) 7)))

(event `ToggleMouse (Client)`
  ;[1 1 1] Inventory
  ;;[1 1 1] Toggle Mouse/Movement
  (`self.Toggle Mouse Cursor`))

(event `EnhancedInput|/Game/SCI/Blueprints/Input/Actions/IA_Inventory`
  (params (ActionValue :type Boolean) (ElapsedSeconds :type "Float (double-precision)") (TriggeredSeconds :type "Float (double-precision)") (InputAction :type "InputAction Object Reference" :default "/Game/SCI/Blueprints/Input/Actions/IA_Inventory.IA_Inventory"))
  ;[1 1 1] Inventory
  ;;[1 1 1] Toggle Inventory
  (:`Started`
    (`/Game/SCI/Blueprints/Components/BPC_InventoryMaster.ToggleContainerUI (Server)` (`self.InventoryMaster`) null 0 "" false)
    (`self.ToggleMouse (Client)`)))

(event `/Game/SCI/Blueprints/Interfaces/BPI_PlayerController.DropItemOnSlot_BPI`
  (params (TargetContainer :type "GameplayTag Structure") (FromContainer :type "GameplayTag Structure") (TargetIndex :type Integer) (FromIndex :type Integer))
  ;[1 1 1] Inventory
  ;;[1 1 1] Item Movement
  (`/Game/SCI/Blueprints/Components/BPC_InventoryMaster.DropItemOnSlot (Server)` (`self.InventoryMaster`) TargetContainer FromContainer TargetIndex FromIndex))

(event `/Game/SCI/Blueprints/Interfaces/BPI_PlayerController.TryMoveItem_BPI`
  (params (ContainerType :type "GameplayTag Structure") (Index :type Integer))
  ;[1 1 1] Inventory
  ;;[1 1 1] Item Movement
  (`/Game/SCI/Blueprints/Components/BPC_InventoryMaster.TryMoveItem (Server)` (`self.InventoryMaster`) ContainerType Index))

(event `/Game/SCI/Blueprints/Interfaces/BPI_PlayerController.ToggleContainerUI_BPI`
  (params (Container :type "/Game/SCI/Blueprints/Actors/BP_ContainerMaster Object Reference") (ContainerSlots :type Integer) (ContainerName :type Text) (IsContainer :type Boolean))
  ;[1 1 1] Inventory
  ;;[1 1 1] Toggle Inventory
  (`/Game/SCI/Blueprints/Components/BPC_InventoryMaster.ToggleContainerUI (Server)` (`self.InventoryMaster`) Container ContainerSlots ContainerName IsContainer)
  (`self.ToggleMouse (Client)`))

(event `/Game/SCI/Blueprints/Interfaces/BPI_PlayerController.DropItem_BPI`
  (params (FromContainer :type "GameplayTag Structure") (FromIndex :type Integer) (Location :type "Vector Structure") (DropAtPlayer :type Boolean))
  ;[1 1 1] Inventory
  ;;[1 1 1] Item Movement
  (`/Game/SCI/Blueprints/Components/BPC_InventoryMaster.DropItem (Server)` (`self.InventoryMaster`) FromContainer FromIndex Location DropAtPlayer (`self.K2_GetPawn`)))

(event `/Game/SCI/Blueprints/Interfaces/BPI_PlayerController.BuyVendorItem_BPI`
  (params (VendorItem :type "/Game/SCI/Blueprints/Structures/STR_VendorItems Structure"))
  ;[1 1 1] Inventory
  ;;[1 1 1] Vendor
  (`/Game/SCI/Blueprints/Components/BPC_InventoryMaster.BuyFromVendor (Server)` (`self.InventoryMaster`) VendorItem))

(event `/Game/SCI/Blueprints/Interfaces/BPI_PlayerController.SendItemsToVendor_BPI`
  (params (Vendor :type "/Game/SCI/Blueprints/Components/BPC_VendorComponent Object Reference"))
  ;[1 1 1] Inventory
  ;;[1 1 1] Vendor
  (`/Game/SCI/Blueprints/Components/BPC_InventoryMaster.SendItemsToVendor (Server)` (`self.InventoryMaster`) Vendor)
  (`self.ToggleMouse (Client)`))

(event `/Game/SCI/Blueprints/Interfaces/BPI_PlayerController.OpenSplitStackUI_BPI`
  (params (ContainerType :type "GameplayTag Structure") (SlotIndex :type Integer))
  ;[1 1 1] Inventory
  ;;[1 1 1] Split Stack
  (`/Game/SCI/Blueprints/Components/BPC_InventoryMaster.OpenSplitStackUI (Server)` (`self.InventoryMaster`) ContainerType SlotIndex))

(event `/Game/SCI/Blueprints/Interfaces/BPI_PlayerController.SplitStack_BPI`
  (params (SplitAmount :type Integer) (ContainerType :type "GameplayTag Structure") (SlotIndex :type Integer))
  ;[1 1 1] Inventory
  ;;[1 1 1] Split Stack
  (`/Game/SCI/Blueprints/Components/BPC_InventoryMaster.SplitStack (Server)` (`self.InventoryMaster`) SplitAmount ContainerType SlotIndex))

(event `/Game/SCI/Blueprints/Interfaces/BPI_PlayerController.RefreshVendorItems_BPI`
  ;[1 1 1] Inventory
  ;;[1 1 1] Vendor
  (`/Game/SCI/Blueprints/Components/BPC_InventoryMaster.RefreshVendorItems (Server)` (`self.InventoryMaster`)))

(fn `GetInteractionTime`
  (returns (TriggerTime :type "Float (double-precision)"))
  (bind _target (`/Game/SCI/Blueprints/Components/BPC_Interact.Target` (`self.InteractionComponent`)))
  ;[1 1 1] Gets the trigger timer for the interaction target if one exists
  (`/Engine/EditorBlueprintResources/StandardMacros.IsValid` (`self.InteractionComponent`)
    (:`Is Valid`
      _)
    (:`Is Not Valid`
      (bind _asbp_player_character (cast `/Game/SCI/Blueprints/Player/BP_PlayerCharacter` (`GameplayStatics.GetPlayerCharacter` 0)))
      (`/Engine/EditorBlueprintResources/StandardMacros.IsValid` _asbp_player_character
        (:`Is Valid`
          (set `self.InteractionComponent` (`/Game/SCI/Blueprints/Player/BP_PlayerCharacter.BPC_Interact` _asbp_player_character))))))
  (`/Engine/EditorBlueprintResources/StandardMacros.IsValid` _target
    (:`Is Valid`
      (bind (_caninteract _triggertime) (message `/Game/SCI/Blueprints/Interfaces/BPI_Interaction.CheckInteractable_BPI` _target))
      (return _triggertime))))

(fn `GetPlayerCharacter_BPI`
  (returns (PlayerCharacter :type "/Game/SCI/Blueprints/Player/BP_PlayerCharacter Object Reference"))
  (return null))

(fn `InitController`
  (bind _returnvalue (pcsubsystem `EnhancedInputLocalPlayerSubsystem` self))
  ;[1 1 1] Registers Enhanced Inputs and enables controls
  (`/Engine/EditorBlueprintResources/StandardMacros.IsValid` _returnvalue
    (:`Is Valid`
      (`EnhancedInputSubsystemInterface.AddMappingContext` _returnvalue "/Game/SCI/Blueprints/Input/IMC_Default.IMC_Default" 0 (struct))
      (set `self.bShowMouseCursor` false)
      (`WidgetBlueprintLibrary.SetInputMode_GameOnly` self true)
      (`self.EnableInput` self))))

(fn `Interact`
  (params (Reset :type Boolean) (InteractTime :type "Float (double-precision)"))
  (bind _interactioncomponent (`self.InteractionComponent`))
  ;[1 1 1] Passes the interaction time to the interaction component or resets it
  (`/Engine/EditorBlueprintResources/StandardMacros.IsValid` (`self.InteractionComponent`)
    (:`Is Valid`
      _)
    (:`Is Not Valid`
      (bind _asbp_player_character (cast `/Game/SCI/Blueprints/Player/BP_PlayerCharacter` (`GameplayStatics.GetPlayerCharacter` 0)))
      (`/Engine/EditorBlueprintResources/StandardMacros.IsValid` _asbp_player_character
        (:`Is Valid`
          (set `self.InteractionComponent` (`/Game/SCI/Blueprints/Player/BP_PlayerCharacter.BPC_Interact` _asbp_player_character))))))
  (if Reset
    (`/Game/SCI/Blueprints/Components/BPC_Interact.ResetInteraction (Client)` _interactioncomponent)
    (`self.ResetInteraction (Server)` (`self.InteractionComponent`))
    (else
      (`/Game/SCI/Blueprints/Components/BPC_Interact.TryInteracting (Client)` _interactioncomponent InteractTime))))

(fn `Toggle Mouse Cursor`
  (bind _returnvalue (`self.K2_GetPawn`))
  ;[1 1 1] Checks if any windows that need the mouse are open and sets the mouse usage accordingly
  (if (not (`self.bShowMouseCursor`))
    (set `self.bShowMouseCursor` true)
    (`WidgetBlueprintLibrary.SetInputMode_GameAndUIEx` self null)
    (`self.DisableInput` _returnvalue self)
    (else
      (set `self.bShowMouseCursor` false)
      (`WidgetBlueprintLibrary.SetInputMode_GameOnly` self)
      (`self.EnableInput` _returnvalue self))))

(fn `TryAddItem_BPI`
  (params (Item :type "/Game/SCI/Blueprints/Structures/STR_ItemData Structure"))
  (returns (Success :type Boolean) (RemainingItems :type Integer))
  (bind (_success _remainingitems) (`/Game/SCI/Blueprints/Components/BPC_InventoryMaster.TryAddItem` (`self.InventoryMaster`) Item))
  (return _success _remainingitems))

(fn `UserConstructionScript`)