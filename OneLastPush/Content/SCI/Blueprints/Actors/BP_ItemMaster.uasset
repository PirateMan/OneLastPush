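; BP_ItemMaster is the base world pickup actor for inventory items, placed in the editor or spawned as a drop.
; A server event fills its item data from a data table row, then sets a replicated mesh whose OnRep enables physics for dropped items.
; Interface calls drive outlining, a name-and-count marker widget, and pickup into the player's inventory.
; Outside debug mode, successful pickups destroy the actor, while failed ones keep the remaining stack count.
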(event `/Game/SCI/Blueprints/Interfaces/BPI_Interaction.SetInteractionText_BPI`
  (bind ((`Name_20_2E0A94954989196EA85027867A65400B` _name) (`CurrentItemValues_57_2158F42247025ADAC852F498D7997C1F` _currentitemvalues)) (break `/Game/SCI/Blueprints/Structures/STR_ItemData` (`self.Item`)))
  ;[1 1 1] World Widget
  (`/Game/SCI/Blueprints/UserInterface/HUD/Misc/UI_Marker.UpdateName` (`self.MarkerWidget`) (`|FormatText` "Pickup {x}x{y}" _name (`.StackCount_2_72BAC6934DA344BFBCF6689B5F9CB7D8` (break `/Game/SCI/Blueprints/Structures/STR_ItemValues` _currentitemvalues))) false))

(event `self.ReceiveBeginPlay`
  ;[1 1 1] World Widget
  (bind _asui_marker (cast `/Game/SCI/Blueprints/UserInterface/HUD/Misc/UI_Marker` (`WidgetComponent.GetWidget` (`self.Marker`))))
  (set `self.MarkerWidget` _asui_marker))

(event `/Game/SCI/Blueprints/Interfaces/BPI_Interaction.LookingAt_BPI`
  (params (LookingAt :type Boolean))
  ;[1 1 1] World Widget
  (`SceneComponent.SetHiddenInGame` (`self.Marker`) (not LookingAt) false))

(event `/Game/SCI/Blueprints/Interfaces/BPI_Interaction.TriggerInteraction_BPI`
  (params (PlayerController :type "PlayerController Object Reference") (PlayerCharacter :type "/Game/SCI/Blueprints/Player/BP_SCIPlayerCharacter Object Reference"))
  (bind _item (`self.Item`))
  ;[1 1 1] Tries to add the item to the players inventory. Updates stack count if not successful (As some items may have been added)
  (bind (_success _remainingitems) (message `/Game/SCI/Blueprints/Interfaces/BPI_PlayerController.TryAddItem_BPI` PlayerController _item))
  (if (`self.DebugItem`)
    _
    (elif _success
      (`self.K2_DestroyActor`)
      (else
        (bind _structout (setmembers `/Game/SCI/Blueprints/Structures/STR_ItemValues` :`StructRef` (`.CurrentItemValues_57_2158F42247025ADAC852F498D7997C1F` (break `/Game/SCI/Blueprints/Structures/STR_ItemData` _item)) :`StackCount` _remainingitems))
        (bind _structout_2 (setmembers `/Game/SCI/Blueprints/Structures/STR_ItemData` :`StructRef` (`self.Item`) :`CurrentItemValues` _structout))
        (set `self.Item` _structout_2)))))

(event `/Game/SCI/Blueprints/Interfaces/BPI_Interaction.SetItemData_BPI`
  (params (ItemHandle :type "DataTableRowHandle Structure") (StackCount :type Integer))
  ;[1 1 1] Sets item data when spawning or loading the item
  (`self.Set Item Data (Server)` ItemHandle StackCount))

(event `Load&SetMesh`
  (bind _value (`BlueprintMapLibrary.Map_Find` (`.StaticMeshes_50_0B10C64340E5133BF8C2769E579D1675` (break `/Game/SCI/Blueprints/Structures/STR_ItemData` (`self.Item`))) "Default"))
  ;[1 1 1] Sets item data when spawning or loading the item
  (`/Engine/EditorBlueprintResources/StandardMacros.IsValid` _value
    (:`Is Valid`
      (set `self.DefaultMesh` _value))))

(event `Set Item Data (Server)`
  (params (ItemHandle :type "DataTableRowHandle Structure") (StackCount :type Integer))
  ;[1 1 1] Sets item data when spawning or loading the item
  (`self.InitItem` ItemHandle StackCount))

(fn `CheckInteractable_BPI`
  (returns (CanInteract :type Boolean) (TriggerTime :type "Float (double-precision)"))
  (return true (`self.Trigger Time`)))

(fn `InitItem`
  (params (ItemHandleRow :type "DataTableRowHandle Structure") (StackCount :type Integer))
  (locals (LocalItem :type "/Game/SCI/Blueprints/Structures/STR_ItemData Structure"))
  ;[1 1 1] Sets up item based on incoming data. Data is comes from the world (if placed in editor) or from a spawn such as item drop.
  (set `self.ItemID` ItemHandleRow)
  (set `local.LocalItem` (`/Game/SCI/Blueprints/Library/Lib_Functions.GetItemDTRow` (`self.ItemID`)))
  (if (`/Game/SCI/Blueprints/Library/Lib_Functions.ItemIsValid` (`local.LocalItem`))
    (bind _structout (setmembers `/Game/SCI/Blueprints/Structures/STR_ItemData` :`StructRef` (`local.LocalItem`) :`CurrentItemValues` (make `/Game/SCI/Blueprints/Structures/STR_ItemValues` StackCount)))
    (set `self.Item` _structout)
    (`self.Load&SetMesh`)))

(fn `OnRep_DefaultMesh`
  (bind _staticmesh (`self.StaticMesh`))
  ;[1 1 1] Sets the mesh for all clients and enables physics if it was dropped
  (`StaticMeshComponent.SetStaticMesh` (`self.StaticMesh`) (`self.DefaultMesh`))
  (if (`self.Dropped`)
    (`PrimitiveComponent.SetCollisionResponseToChannel` _staticmesh "ECC_Visibility" "ECR_Block")
    (`PrimitiveComponent.SetSimulatePhysics` _staticmesh true)))

(fn `ShouldOutline_BPI`
  (returns (Outline :type Boolean))
  (return true))

(fn `UserConstructionScript`
  (if (not (`self.Dropped`))
    (`self.Set Item Data (Server)` (`self.ItemID`) (`self.Stack Count`))))