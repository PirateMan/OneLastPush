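; Blueprint function library of shared helpers for data-table-backed items and gameplay tag display names.
; Item helpers fetch a handle's row after checking its table and row name, treat an item as valid when its row name is set, and compare handles by table and row.
; AddSpaceToTags strips a parent tag and splits words at capitals, detected by comparison with a lowercased copy, to produce spaced UI text.
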(fn `AddSpaceToTags`
  (params (Tag :type "GameplayTag Structure (by ref)") (ParentTag :type "GameplayTag Structure (by ref)"))
  (returns (Output :type Text))
  (locals (InputString :type String) (OriginalArray :type "Array of String") (LowerCaseOnlyArray :type "Array of String") (OutputString :type String) (SpaceCharacter :type String) (ArrayOfIndividualWords :type "Array of String") (LocalIndividualWordNumber :type Integer) (InputString :type String))
  (bind _localindividualwordnumber (`local.LocalIndividualWordNumber`))
  (bind _arrayofindividualwords (`local.ArrayOfIndividualWords`))
  ;[1 1 1] Used to return a Gameplay Tags name for the UI. Takes the incoming tag, remove it's parent (i.e. Player.Attribute.MaxHealth becomes MaxHealth). Then, using capital letters, adds spaces (i.e. MaxHealth becomes Max Health) before returning it as a "Text" variable.
  (set `local.InputString` (`KismetStringLibrary.Conv_NameToString` (`BlueprintGameplayTagLibrary.GetTagName` Tag)))
  (`KismetStringLibrary.ReplaceInline` (`local.InputString`) (`KismetStringLibrary.Conv_NameToString` (`BlueprintGameplayTagLibrary.GetTagName` ParentTag)))
  (set `local.OriginalArray` (`KismetStringLibrary.GetCharacterArrayFromString` (`local.InputString`)))
  (set `local.LowerCaseOnlyArray` (`KismetStringLibrary.GetCharacterArrayFromString` (`KismetStringLibrary.ToLower` (`local.InputString`))))
  (for (_array_element _array_index) (`local.OriginalArray`)
    (if (`KismetStringLibrary.EqualEqual_StrStr` _array_element (`|GetArrayItem` (`local.LowerCaseOnlyArray`) _array_index))
      (if (`KismetArrayLibrary.Array_IsValidIndex` _arrayofindividualwords _localindividualwordnumber)
        (`KismetArrayLibrary.Array_Set` (`local.ArrayOfIndividualWords`) (`local.LocalIndividualWordNumber`) (`KismetStringLibrary.Concat_StrStr` (`|GetArrayItem` _arrayofindividualwords _localindividualwordnumber) _array_element)))
      (else
        (bind _returnvalue (`KismetArrayLibrary.Array_Add` (`local.ArrayOfIndividualWords`) _array_element))
        (set `local.LocalIndividualWordNumber` _returnvalue))))
  (bind _output_get (set `local.OutputString` (`KismetStringLibrary.JoinStringArray` (`local.ArrayOfIndividualWords`) (`local.SpaceCharacter`))))
  (return (`KismetTextLibrary.Conv_StringToText` _output_get)))

(fn `GetItemDTRow`
  (params (Handle :type "DataTableRowHandle Structure (by ref)"))
  (returns (Row :type "/Game/SCI/Blueprints/Structures/STR_ItemData Structure"))
  (bind (_datatable _rowname) (break `DataTableRowHandle` Handle))
  (if (and (`KismetSystemLibrary.IsValid` _datatable) (!= _rowname "None"))
    (bind _returnvalue (`|GetDataTableRow` _datatable _rowname)
      (:`then`
        (return _returnvalue)))))

(fn `HandlesAreEqual`
  (params (HandleA :type "DataTableRowHandle Structure (by ref)") (HandleB :type "DataTableRowHandle Structure (by ref)"))
  (returns (Equal :type Boolean))
  (bind (_datatable _rowname) (break `DataTableRowHandle` HandleA))
  (bind (_datatable_2 _rowname_2) (break `DataTableRowHandle` HandleB))
  (return (and (== _datatable _datatable_2) (== _rowname _rowname_2))))

(fn `ItemIsValid`
  (params (Item :type "/Game/SCI/Blueprints/Structures/STR_ItemData Structure (by ref)"))
  (returns (Valid :type Boolean))
  (return (!= (`.RowName` (break `DataTableRowHandle` (`.Handle_35_D3E721B346F521CA8513EDBFB73D1638` (break `/Game/SCI/Blueprints/Structures/STR_ItemData` Item)))) "None")))