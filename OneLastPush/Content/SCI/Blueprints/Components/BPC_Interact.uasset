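; Player interaction component that finds, highlights and triggers interactable actors through BPI_Interaction.
; On the local controller, a looping timer traces from the camera, keeps in-range hits as the target, notifies look-at changes and toggles custom-depth outlines.
; Interaction attempts update hold progress on the owner's UI and go to the server, which re-traces and triggers the target once its required time elapses, latched until reset.
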(event `TryInteracting (Client)`
  (params (InteractTime :type "Float (double-precision)"))
  (bind _target (`self.Target`))
  (bind _target_2 (`self.Target`))
  ;[1 1 1] Checks if the Target is an interactable object and passing the Trigger Interaction BPI after the trigger time defined for that interactable object.
  (if (and (`KismetSystemLibrary.IsValid` _target) (`KismetSystemLibrary.DoesImplementInterface` _target "/Game/SCI/Blueprints/Interfaces/BPI_Interaction.BPI_Interaction_C"))
    (`self.TryInteracting (Server)` InteractTime)
    (`/Engine/EditorBlueprintResources/StandardMacros.IsValid` _target_2
      (:`Is Valid`
        (bind (_caninteract _triggertime) (message `/Game/SCI/Blueprints/Interfaces/BPI_Interaction.CheckInteractable_BPI` _target_2))
        (if true
          (message `/Game/SCI/Blueprints/Interfaces/BPI_PlayerCharacter.UpdateInteractUI_BPI` (`self.GetOwner`) (/ InteractTime _triggertime)))))))

(event `self.ReceiveBeginPlay`
  ;[1 1 1] Sets the Interaction Tick using a timer.
  (`KismetSystemLibrary.K2_SetTimerDelegate` (delegate `InteractionTick`) 0.2 true))

(event `ResetInteraction`
  ;[1 1 1] Checks if the Target is an interactable object and passing the Trigger Interaction BPI after the trigger time defined for that interactable object.
  (set `self.Triggered` false))

(event `InteractionTick`
  ;[1 1 1] Sets the Interaction Tick using a timer.
  (if (`self.IsLocalController`)
    (`self.UpdateTarget`)
    (`self.Set Look At`)))

(event `TryInteracting (Server)`
  (params (InteractTime :type "Float (double-precision)"))
  (bind _target (`self.Target`))
  ;[1 1 1] Checks if the Target is an interactable object and passing the Trigger Interaction BPI after the trigger time defined for that interactable object.
  (`self.UpdateTarget`)
  (if (not (`self.Triggered`))
    (bind (_caninteract _triggertime) (message `/Game/SCI/Blueprints/Interfaces/BPI_Interaction.CheckInteractable_BPI` _target))
    (if (and _caninteract (>= InteractTime _triggertime))
      (set `self.Triggered` true)
      (message `/Game/SCI/Blueprints/Interfaces/BPI_Interaction.TriggerInteraction_BPI` _target (`self.Player Controller`) (`self.Player Character`))
      (set `self.Target` null))))

(event `ResetInteraction (Client)`
  ;[1 1 1] Checks if the Target is an interactable object and passing the Trigger Interaction BPI after the trigger time defined for that interactable object.
  (message `/Game/SCI/Blueprints/Interfaces/BPI_PlayerCharacter.UpdateInteractUI_BPI` (`self.GetOwner`) 0.0))

(fn `InitComponent`
  (params (PlayerController :type "PlayerController Object Reference") (PlayerCharacter :type "/Game/SCI/Blueprints/Player/BP_SCIPlayerCharacter Object Reference"))
  (set `self.Player Character` PlayerCharacter)
  (`/Engine/EditorBlueprintResources/StandardMacros.IsValid` PlayerController
    (:`Is Valid`
      (bind _output_get (set `self.Player Controller` PlayerController))
      (set `self.IsLocalController` (`KismetSystemLibrary.IsValid` (`PlayerController.GetHUD` _output_get))))))

(fn `Set Look At`
  (bind _target (`self.Target`))
  (bind _target_2 (`self.Target`))
  (bind _target_3 (`self.Target`))
  (bind _previoustarget (`self.PreviousTarget`))
  ;[1 1 1] Checks if the target should be outlined and outlines it if it should. If the target is no longer valid or the new target should not be outlined, removes the outline from the previous target.
  (`/Engine/EditorBlueprintResources/StandardMacros.IsValid` _target
    (:`Is Valid`
      (if (not (== _target (`self.PreviousTarget`)))
        (`/Engine/EditorBlueprintResources/StandardMacros.IsValid` _previoustarget :!label _label
          (:`Is Valid`
            (message `/Game/SCI/Blueprints/Interfaces/BPI_Interaction.LookingAt_BPI` _previoustarget false)
            (for _array_element (`Actor.K2_GetComponentsByClass` _previoustarget "/Script/Engine.PrimitiveComponent")
              (`PrimitiveComponent.SetRenderCustomDepth` _array_element false)
              (`PrimitiveComponent.SetCustomDepthStencilValue` _array_element 1)))
          (:`Is Not Valid`
            _))
        (`/Engine/EditorBlueprintResources/StandardMacros.IsValid` _target_2
          (:`Is Valid`
            (message `/Game/SCI/Blueprints/Interfaces/BPI_Interaction.LookingAt_BPI` _target_2 true)
            (message `/Game/SCI/Blueprints/Interfaces/BPI_Interaction.SetInteractionText_BPI` _target_2)
            (set `self.PreviousTarget` _target_3)
            (bind _outline (message `/Game/SCI/Blueprints/Interfaces/BPI_Interaction.ShouldOutline_BPI` _target_3))
            (if _outline
              (for _array_element_2 (`Actor.K2_GetComponentsByClass` _target_3 "/Script/Engine.PrimitiveComponent")
                (`PrimitiveComponent.SetRenderCustomDepth` _array_element_2 true)
                (`PrimitiveComponent.SetCustomDepthStencilValue` _array_element_2 1))))
          (:`Is Not Valid`
            (set `self.PreviousTarget` null)))))
    (:`Is Not Valid`
      (goto _label))))

(fn `SetTarget`
  (params (NewTarget :type "Actor Object Reference"))
  ;[1 1 1] Sets the target and calls "On Target Changed"
  (if (!= NewTarget (`self.Target`))
    (set `self.Target` NewTarget)))

(fn `TickTrace`
  (returns (HitResult :type "HitResult Structure"))
  (bind _playercameramanager (`PlayerController.PlayerCameraManager` (`self.Player Controller`)))
  (bind _returnvalue (`PlayerCameraManager.GetCameraLocation` _playercameramanager))
  ;[1 1 1] Fires a trace from the camera that is looking for a new target.
  (bind _outhit (`KismetSystemLibrary.LineTraceSingle` _returnvalue (+ _returnvalue (* (`KismetMathLibrary.GetForwardVector` (`PlayerCameraManager.GetCameraRotation` _playercameramanager)) (`self.TraceDistance`))) "TraceTypeQuery1" false (`|MakeArray` (`Controller.K2_GetPawn` (`self.Player Controller`)) :!type "Actor Object Reference")))
  (return _outhit))

(fn `UpdateTarget`
  ;[1 1 1] Performs the Tick Trace and updates the Target if in range and hit.
  (`/Engine/EditorBlueprintResources/StandardMacros.IsValid` (`Controller.K2_GetPawn` (`self.Player Controller`))
    (:`Is Valid`
      (bind _hitresult (`self.TickTrace`))
      (bind (_bblockinghit _binitialoverlap _time _distance _location _impactpoint _normal _impactnormal _physmat _hitactor) (`GameplayStatics.BreakHitResult` _hitresult))
      (if _bblockinghit
        (set `self.Impact Normal` _impactnormal)
        (if (<= (`KismetMathLibrary.VSize` (- _location (`Actor.K2_GetActorLocation` (`Controller.K2_GetPawn` (`self.Player Controller`))))) (`self.HitDistance`))
          (`self.SetTarget` _hitactor)
          (else
            (`self.SetTarget` null :!label _label)))
        (else
          (goto _label))))))