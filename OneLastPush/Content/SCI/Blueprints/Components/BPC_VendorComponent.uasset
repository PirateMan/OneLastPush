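; Vendor component that supplies an item list to player controllers and tracks its stock.
; On BeginPlay it loads the list from a data table row and builds cost entries with item indexes, merging matching cost items only when the cost count is zero.
; Toggling sends the component to a controller through Blueprint interface messages.
; Purchases subtract from the stack count, then every controller in its list is told to refresh.
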(event `self.ReceiveBeginPlay`
  (bind (_vendorhandle_datatable _vendorhandle_rowname) (break `DataTableRowHandle` (`self.VendorHandle`)))
  ;[1 1 1] Sets up the vendor on begin play
  (bind _returnvalue (`|GetDataTableRow` _vendorhandle_datatable _vendorhandle_rowname)
    (:`then`
      (set `self.VendorList` _returnvalue)
      (`self.GetUniqueCosts`))))

(event `ToggleVendor`
  (params (Controller :type "Controller Object Reference"))
  ;[1 1 1] Toggles the vendor and UI for it
  (message `/Game/SCI/Blueprints/Interfaces/BPI_PlayerController.SendItemsToVendor_BPI` Controller self))

(event `RemoveController (Server)`
  (params (Item :type "Controller Object Reference (by ref)"))
  ;[1 1 1] Removes a controller from the vendor
  (`KismetArrayLibrary.Array_RemoveItem` (`self.Controllers`) Item))

(event `UpdateVendor`
  (params (VendorIndex :type Integer))
  (bind ((`VendorItems_10_FFE17E6E4C145C64E1F3D8A18645428B` _vendoritems)) (break `/Game/SCI/Blueprints/Structures/STR_Vendors` (`self.VendorList`)))
  (bind _output (`|GetArrayItem` _vendoritems VendorIndex))
  (bind ((`StackCount_23_1420D36F4A0CF9B9D76F46A8E385AE0B` _stackcount) (`PurchaseCount_22_1F6A2FDE440273D7332AC58DD313A380` _purchasecount)) (break `/Game/SCI/Blueprints/Structures/STR_VendorItems` _output))
  ;[1 1 1] Updates the vendors stock count after purchase
  (set `self.VendorItems` _vendoritems)
  (bind _structout (setmembers `/Game/SCI/Blueprints/Structures/STR_VendorItems` :`StructRef` _output :`StackCount` (- _stackcount _purchasecount)))
  (`KismetArrayLibrary.Array_Set` (`self.VendorItems`) VendorIndex _structout)
  (setmembers `/Game/SCI/Blueprints/Structures/STR_Vendors` :`StructRef` (`self.VendorList`) :`VendorItems` (`self.VendorItems`))
  (for _array_element (`self.Controllers`)
    (message `/Game/SCI/Blueprints/Interfaces/BPI_PlayerController.RefreshVendorItems_BPI` _array_element)))

(fn `GetUniqueCosts`
  (locals (LocalFound :type Boolean) (LocalIndexes :type "Array of Integer") (LocalVendorItems :type "Array of /Game/SCI/Blueprints/Structures/STR_VendorItems Structure") (LocalCostDetails :type "/Game/SCI/Blueprints/Structures/STR_VendorCost Structure"))
  (bind _localindexes (`local.LocalIndexes`))
  (bind (_costitem _costcount _indexes) (break `/Game/SCI/Blueprints/Structures/STR_VendorCost` (`local.LocalCostDetails`)))
  ;[1 1 1] Gets each unique cost item and adds it to the Local Cost Items array with all of the Indexes it applies to
  (bind _output_get (set `local.LocalVendorItems` (`.VendorItems_10_FFE17E6E4C145C64E1F3D8A18645428B` (break `/Game/SCI/Blueprints/Structures/STR_Vendors` (`self.VendorList`)))))
  (for (_array_element _array_index) _output_get
    (set `local.LocalFound` false)
    (for (_array_element_2 _array_index_2) (`self.UniqueCostItems`)
      (set `local.LocalCostDetails` _array_element_2)
      (set `local.LocalIndexes` _indexes)
      (bind ((`CostItem_21_4843DADC4DA9386EEDE59D99B91D54A1` _costitem_2) (`CostCount_19_83A89768423344C90D1B68BA4C0A6E4E` _costcount_2)) (break `/Game/SCI/Blueprints/Structures/STR_VendorItems` _array_element))
      (if (and (`/Game/SCI/Blueprints/Library/Lib_Functions.HandlesAreEqual` _costitem _costitem_2) (== 0 _costcount_2))
        (`KismetArrayLibrary.Array_Add` _localindexes _array_index)
        (bind _structout (setmembers `/Game/SCI/Blueprints/Structures/STR_VendorCost` :`StructRef` (`local.LocalCostDetails`) :`Indexes` _localindexes))
        (`KismetArrayLibrary.Array_Set` (`self.UniqueCostItems`) _array_index_2 _structout)
        (set `local.LocalFound` true)
        (else
          (set `local.LocalFound` false))))
    (if (not (`local.LocalFound`))
      (`KismetArrayLibrary.Array_Add` (`self.UniqueCostItems`) (make `/Game/SCI/Blueprints/Structures/STR_VendorCost` _costitem_2 _costcount_2 (`|MakeArray` _array_index))))))