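; Inventory child of a container component that stores currency items as amounts in a tag-keyed Currencies map instead of as items.
; Adding an item and checking requirements branch on the Currency type tag, deferring to the parent for everything else.
; Spending looks up the item's data table row and deducts from the map if the balance suffices.
; Slot drops run the parent logic first, then transfer the item if it returns false.
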(fn `AddItemToContainer`
  (params (Item :type "/Game/SCI/Blueprints/Structures/STR_ItemData Structure (by ref)"))
  (returns (Success :type Boolean) (AddedItems :type Integer) (RemainingItems :type Integer))
  (bind ((`Type_36_39F9A1D94F257757400C869236547834` _type) (`CurrentItemValues_57_2158F42247025ADAC852F498D7997C1F` _currentitemvalues)) (break `/Game/SCI/Blueprints/Structures/STR_ItemData` Item))
  (bind _stackcount (break `/Game/SCI/Blueprints/Structures/STR_ItemValues` _currentitemvalues))
  ;[1 1 1] If the item incoming to the inventory is a currency, adds it as one instead of as an item.
  (if (`BlueprintGameplayTagLibrary.MatchesTag` _type (struct :`TagName` "Items.Type.Currency"))
    (bind _updateditem (`self.AddCurrency` _type _stackcount (`local.Item`)))
    (`self.OnItemChanged` _updateditem true)
    (return true _stackcount 0)
    (else
      (bind (_success _addeditems _remainingitems) (`parent.AddItemToContainer` Item))
      (return _success _addeditems _remainingitems))))

(fn `Check Has Enough`
  (params (RequiredItem :type "/Game/SCI/Blueprints/Structures/STR_ItemData Structure") (Quantity :type Integer))
  (returns (HasEnough :type Boolean) (AmountFound :type Integer))
  (bind ((`Type_36_39F9A1D94F257757400C869236547834` _type)) (break `/Game/SCI/Blueprints/Structures/STR_ItemData` RequiredItem))
  (bind (_value _returnvalue) (`BlueprintMapLibrary.Map_Find` (`self.Currencies`) _type))
  ;[1 1 1] Checks if the incoming requirement is a currency and if so, if you have enough. Only applies to inventory.
  (if (`BlueprintGameplayTagLibrary.MatchesTag` _type (struct :`TagName` "Items.Type.Currency"))
    (if _returnvalue
      (return (>= _value (`local.Quantity`)) 0)
      (else
        (return false 0)))
    (else
      (bind (_hasenough _amountfound) (`parent.Check Has Enough` (`local.RequiredItem`) (`local.Quantity`)))
      (return _hasenough _amountfound))))

(fn `Drop Item on Slot`
  (params (FromContainer :type "/Game/SCI/Blueprints/Components/BPC_Container Object Reference") (TargetIndex :type Integer) (FromIndex :type Integer))
  ;[1 1 1] After running parent function, transfers the item
  (bind _sameslot (`parent.Drop Item on Slot` FromContainer TargetIndex FromIndex))
  (if (not _sameslot)
    (`self.Transfer Item` FromContainer self TargetIndex FromIndex)))

(fn `LoadPlayerData_BPI`
  (returns (Success :type Boolean)))

(fn `SavePlayerData_BPI`
  (returns (Success :type Boolean)))

(fn `Spend Currency`
  (params (CurrencyItem :type "DataTableRowHandle Structure") (AmountToSpend :type Integer))
  (returns (Success :type Boolean) (Currency :type "GameplayTag Structure") (UpdatedAmount :type Integer))
  (locals (LocalCurrencyItem :type "/Game/SCI/Blueprints/Structures/STR_ItemData Structure"))
  (bind ((`Type_36_39F9A1D94F257757400C869236547834` _type)) (break `/Game/SCI/Blueprints/Structures/STR_ItemData` (`local.LocalCurrencyItem`)))
  (bind (_value _returnvalue) (`BlueprintMapLibrary.Map_Find` (`self.Currencies`) _type))
  ;[1 1 1] Checks if you have the currency and enough of it and if so spends it.
  (set `local.LocalCurrencyItem` (`self.GetItemRowFromDT` CurrencyItem))
  (if _returnvalue
    (if (>= _value (`local.AmountToSpend`))
      (`BlueprintMapLibrary.Map_Add` (`self.Currencies`) _type (- _value (`local.AmountToSpend`)))
      (return true _type (`BlueprintMapLibrary.Map_Find` (`self.Currencies`) _type))
      (else
        _)))
  (return false (struct) 0))