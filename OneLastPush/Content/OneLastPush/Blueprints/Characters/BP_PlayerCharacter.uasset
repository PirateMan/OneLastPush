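; Player character Blueprint for OneLastPush that routes touch input to actions and adds a time-dilation effect when the character is damaged.
; Touch events forward to move, aim, AoE attack and dash functions defined outside this graph, swapping X and Y on both stick axes.
; The damage event plays a Timeline that drives global time dilation each update and restores normal speed when it finishes.
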(event `CustomEvent_3`
  ;[1 1 1] Touch Inputs
  (`self.DoAoEAttack`))

(event `CustomEvent_4`
  ;[1 1 1] Touch Inputs
  (`self.DoDash`))

(event `CustomEvent_2`
  (params (Axis :type "Vector2D Structure") (Axis_X :type "Float (double-precision)") (Axis_Y :type "Float (double-precision)"))
  ;[1 1 1] Touch Inputs
  (`self.DoMove` Axis_Y Axis_X))

(event `CustomEvent_1`
  (params (Axis :type "Vector2D Structure") (Axis_X :type "Float (double-precision)") (Axis_Y :type "Float (double-precision)"))
  ;[1 1 1] Touch Inputs
  (`self.DoAim` Axis_Y Axis_X))

(event `CustomEvent`
  ;[1 1 1] Apply time dilation when the player character is damaged
  (bind (_direction _time_dilation) (`Timeline|Timeline` :!via `PlayFromStart`)
    (:`Update`
      (`GameplayStatics.SetGlobalTimeDilation` _time_dilation))
    (:`Finished`
      (`GameplayStatics.SetGlobalTimeDilation` 1.0))))

(fn `UserConstructionScript`)